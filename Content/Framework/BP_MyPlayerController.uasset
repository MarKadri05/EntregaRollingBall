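; BP_MyPlayerController is a player controller that manages the game's HUD and end-of-level victory screen.
; On BeginPlay it creates WBP_MainWidget and displays the current lives and score.
; Update events receive new lives, score and time values and write formatted text directly into that widget's text blocks.
; ShowVictoryScreen spawns WBP_VictoryWidget and passes it the final score, time, coins and leaderboard.
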(event `self.ReceiveBeginPlay`
  ; UI de score y vidas
  (`self.InitWidget`)
  (`self.SetUILives` (`self.CurrentLives`))
  (`self.SetUIScore` (`self.CurrentScore`)))

(event `self.UpdateUILives`
  (params (NewLives :type Integer))
  ; Actualizar vidas
  (`self.SetUILives` NewLives))

(event `self.UpdateUIScore`
  (params (NewScore :type Integer))
  ; Actualizar puntuación
  (`self.SetUIScore` NewScore))

(event `self.UpdateUITimer`
  (params (Minutes :type Integer) (Seconds :type Integer))
  ; Actualizar contador de tiempo
  (`self.UpdateTimer` Minutes Seconds))

(event `self.ShowVictoryScreen`
  (params (FinalScore :type Integer) (FinalTime :type Integer) (FinalCoins :type Integer) (Leaderboard :type "Array of ScoreEntry Structure (by ref)"))
  ; Pantalla de victoria al finalizar el nivel
  (bind _returnvalue (`|CreateWidget` "/Game/UI/WBP_VictoryWidget.WBP_VictoryWidget_C"))
  (`UserWidget.AddToViewport` _returnvalue 0)
  (`/Game/UI/WBP_VictoryWidget.InitVictoryScreen` _returnvalue FinalTime FinalScore FinalCoins Leaderboard))

(fn `InitWidget`
  (bind _returnvalue (`|CreateWidget` "/Game/UI/WBP_MainWidget.WBP_MainWidget_C" self))
  (bind _output_get (set `self.MainWidget` _returnvalue))
  (`UserWidget.AddToViewport` _output_get 0))

(fn `SetUILives`
  (params (Lives :type Integer))
  (`TextBlock.SetText` (`/Game/UI/WBP_MainWidget.LivesText` (`self.MainWidget`)) (`KismetTextLibrary.Conv_StringToText` (`KismetStringLibrary.Concat_StrStr` "Lives: " (`KismetStringLibrary.Conv_IntToString` Lives)))))

(fn `SetUIScore`
  (params (Score :type Integer))
  (`TextBlock.SetText` (`/Game/UI/WBP_MainWidget.ScoreText` (`self.MainWidget`)) (`KismetTextLibrary.Conv_StringToText` (`KismetStringLibrary.Concat_StrStr` "Score: " (`KismetStringLibrary.Conv_IntToString` Score)))))

(fn `UpdateLives`
  (`TextBlock.SetText` (`/Game/UI/WBP_MainWidget.LivesText` (`self.MainWidget`)) (`KismetTextLibrary.Conv_StringToText` (`KismetStringLibrary.Concat_StrStr` "Lives: " (`KismetStringLibrary.Conv_IntToString` 0)))))

(fn `UpdateTimer`
  (params (Value :type Integer) (Value2 :type Integer))
  (`TextBlock.SetText` (`/Game/UI/WBP_MainWidget.TimerText` (`self.MainWidget`)) (`|FormatText` "{0}:{1}" (`|GenericToText` Value) (`|GenericToText` Value2))))

(fn `UserConstructionScript`)